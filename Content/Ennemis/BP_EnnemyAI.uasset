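; Enemy AI Blueprint that chases the player on sight and plays a melee attack animation on reaching them.
; PawnSensing sets a seen flag, never cleared here, and calls FollowPlayer, which uses AI MoveTo toward player character 0.
; On arrival, a CanAttack flag gates the montage and resets after a delay of its length, though each FollowPlayer call also resets it.
; No damage is applied in this graph.
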(event OnSeePawn(PawnSensing)
  (params (Pawn :type Pawn%20Object%20Reference))
  (bind _output_get (Variables|Default|SetIsSeeingPlayer?%20 true))
  (if _output_get
    (CallFunction|FollowPlayer)))

(event Custom|FollowPlayer
  (Variables|Default|SetCanAttack? true)
  (if (Variables|Default|GetIsSeeingPlayer?%20)
    (AI|AIMoveTo self "0, 0, 0" (Game|GetPlayerCharacter 0) 7e+01 false
      (:OnSuccess
        (Development|PrintString "Hello")
        (if (Variables|Default|GetCanAttack?)
          (Variables|Default|SetCanAttack? false)
          (bind _returnvalue (Animation|PlayAnimMontage self "/Game/Ennemis/Animation/AI/AI_AttackAnim.AI_AttackAnim" 1.0 "None"))
          (Utilities|FlowControl|Delay _returnvalue)
          (Variables|Default|SetCanAttack? true))))))

(event EventBeginPlay)

(event Collision|EventActorBeginOverlap
  (params (OtherActor :type Actor%20Object%20Reference)))

(event EventTick
  (params (DeltaSeconds :type Float%20%28single-precision%29)))

(fn ConstructionScript)