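; Test AI for the boss mecha that chases the player and shakes the camera at close range.
; PawnSensing sets a seen flag, which is never cleared, and issues an AI MoveTo toward the player character.
; A sphere overlap toggles a flag that makes Tick play the mecha camera shake every frame at the player's follow camera.
; GetPath is an empty stub.
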(event OnSeePawn(PawnSensing)
  (params (Pawn :type Pawn%20Object%20Reference))
  (Variables|Default|SetIsSeeingPlayer true)
  (CallFunction|FollowPlayer))

(event OnComponentBeginOverlap(Sphere)
  (params (OverlappedComponent :type Primitive%20Component%20Object%20Reference) (OtherActor :type Actor%20Object%20Reference) (OtherComp :type Primitive%20Component%20Object%20Reference) (OtherBodyIndex :type Integer) (bFromSweep :type Boolean) (SweepResult :type Hit%20Result%20Structure%20%28by%20ref%29))
  (bind _asbp_third_person_character (Utilities|Casting|CastToBP_ThirdPersonCharacter OtherActor))
  (Variables|Default|SetAs%20BP%20Third%20Person%20Character _asbp_third_person_character)
  (Variables|Default|SetCheckIn true))

(event OnComponentEndOverlap(Sphere)
  (params (OverlappedComponent :type Primitive%20Component%20Object%20Reference) (OtherActor :type Actor%20Object%20Reference) (OtherComp :type Primitive%20Component%20Object%20Reference) (OtherBodyIndex :type Integer))
  (bind _asbp_third_person_character (Utilities|Casting|CastToBP_ThirdPersonCharacter OtherActor))
  (Variables|Default|SetAs%20BP%20Third%20Person%20Character _asbp_third_person_character)
  (Variables|Default|SetCheckIn false))

(event Custom|Follow%20player
  (if (Variables|Default|GetIsSeeingPlayer)
    (AI|AIMoveTo (stale OnSeePawn(PawnSensing) Pawn) "0, 0, 0" (Game|GetPlayerCharacter 0) 5.0 false)))

(event EventTick
  (params (DeltaSeconds :type Float%20%28single-precision%29))
  (if (Variables|Default|GetCheckIn)
    (Camera|PlayWorldCameraShake "/Game/Boss_Mecha/CS_Mecha.CS_Mecha_C" (Transformation|GetWorldLocation (Variables|/Game/Controls/Blueprints/BP_ThirdPersonCharacter.BP_ThirdPersonCharacter_C|GetFollowCamera (Variables|Default|GetAs%20BP%20Third%20Person%20Character))) 1e+03 1.5e+03)))

(fn ConstructionScript)

(fn GetPath
  (params (Splines :type Array%20of%20Path%20Object%20References)))