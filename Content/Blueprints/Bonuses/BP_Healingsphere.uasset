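; BP_Healingsphere is a health pickup that heals the player on overlap and then destroys itself.
; When the player pawn overlaps it, GainHealth adds a fixed amount to Health stored on the Game_Instance, clamped between zero and MaxHealth.
; It also prints the new health value to the screen before being destroyed.
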(event Custom|GainHealth
  (params (GainedHealth :type Float%20%28double-precision%29))
  (bind _asgame_instance (Utilities|Casting|CastToGame_Instance (Game|GetGameInstance)))
  (bind _output_get (Variables|Default|SetGI_Ref _asgame_instance))
  (Variables|/Game/Blueprints/Game_Instance.Game_Instance_C|SetHealth _output_get (Math|Float|Clamp(Float) (+ (Variables|/Game/Blueprints/Game_Instance.Game_Instance_C|GetHealth (Variables|Default|GetGI_Ref)) GainedHealth) 0.0 (Variables|/Game/Blueprints/Game_Instance.Game_Instance_C|GetMaxHealth (Variables|Default|GetGI_Ref)))))

(event EventBeginPlay)

(event Collision|EventActorBeginOverlap
  (params (OtherActor :type Actor%20Object%20Reference))
  (if (== (Game|Player|GetPlayerPawn 0) OtherActor)
    (CallFunction|GainHealth 2e+01)
    (Development|PrintString (Utilities|String|ToString(Float) (Variables|/Game/Blueprints/Game_Instance.Game_Instance_C|GetHealth (Variables|Default|GetGI_Ref))))
    (Actor|DestroyActor)))

(event EventTick
  (params (DeltaSeconds :type Float%20%28single-precision%29)))

(fn ConstructionScript)