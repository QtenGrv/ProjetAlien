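; Loot spawner actor that spawns a Loot_ItemBP at its own location every second on a looping timer.
; Each spawn passes item details built from a rarity picked by ChooseRarity.
; ChooseRarity does a weighted random roll over the RarityMap in the Loot_Instance game instance, subtracting weights until the roll lands.
; The weight total, roll and chosen rarity are printed for debugging.
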(event Custom|CreateLoot
  (bind _rarity (CallFunction|ChooseRarity))
  (Game|SpawnActorfromClass "/Game/Blueprints/Bonuses/Loot_ItemBP.Loot_ItemBP_C" (Math|Conversions|ToTransform(Vector) (Transformation|GetActorLocation)) "Undefined" "MultiplyWithRoot" 0 (Utilities|Struct|MakeItem_Struct _rarity) 0))

(event EventBeginPlay
  (Utilities|Time|SetTimerbyEvent (delegate Custom|CreateLoot) 1.0 true))

(event Collision|EventActorBeginOverlap
  (params (OtherActor :type Actor%20Object%20Reference)))

(event EventTick
  (params (DeltaSeconds :type Float%20%28single-precision%29)))

(fn ConstructionScript)

(fn ChooseRarity
  (bind _asloot_instance (Utilities|Casting|CastToLoot_Instance (Game|GetGameInstance)))
  (bind _keys (Utilities|Map|Keys (Variables|/Game/Blueprints/Bonuses/Loot_Instance.Loot_Instance_C|GetRarityMap _asloot_instance)))
  (for _array_element _keys
    (LocalVariables|SetSumOfRarities (+ (.Value (Utilities|Map|Find (Variables|/Game/Blueprints/Bonuses/Loot_Instance.Loot_Instance_C|GetRarityMap _asloot_instance) _array_element)) (LocalVariables|GetSumOfRarities))))
  (LocalVariables|SetLootRoll (Math|Random|RandomFloatinRange 0.0 (LocalVariables|GetSumOfRarities)))
  ;[1 1 1] Debug
  (Development|PrintString (Utilities|String|ToString(Float) (LocalVariables|GetSumOfRarities)))
  (Development|PrintString (Utilities|String|ToString(Float) (LocalVariables|GetLootRoll)))
  (Utilities|Map|Keys (Variables|/Game/Blueprints/Bonuses/Loot_Instance.Loot_Instance_C|GetRarityMap _asloot_instance))
  (bind _array_element_2 (Utilities|Array|ForEachLoopwithBreak "NewEnumerator0" :!label _label)
    (:LoopBody
      (if (>= (.Value (Utilities|Map|Find (Variables|/Game/Blueprints/Bonuses/Loot_Instance.Loot_Instance_C|GetRarityMap _asloot_instance) _array_element_2)) (LocalVariables|GetLootRoll))
        (LocalVariables|SetRarityOut _array_element_2)
        (goto _label Break)
        (else
          (LocalVariables|SetLootRoll (- (LocalVariables|GetLootRoll) (.Value (Utilities|Map|Find (Variables|/Game/Blueprints/Bonuses/Loot_Instance.Loot_Instance_C|GetRarityMap _asloot_instance) _array_element_2)))))))
    (:Completed
      (Development|PrintString (Utilities|String|EnumtoString (LocalVariables|GetRarityOut)))
      (return (LocalVariables|GetRarityOut)))))