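; Homing missile for the Mecha boss that chases the player and explodes with damage, camera shake, particles and sound.
; A looping timer turns its yaw toward the player, while a half-second loop refreshes the projectile's homing target on the player pawn.
; Box overlaps sphere-trace for the player; Pillar contact or a 15-second lifetime calls EXPLOSION, which sphere-traces for pawns, ignoring Mecha-tagged actors, and only takes effect on a hit.
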(event OnComponentBeginOverlap(Box)
  (params (OverlappedComponent :type Primitive%20Component%20Object%20Reference) (OtherActor :type Actor%20Object%20Reference) (OtherComp :type Primitive%20Component%20Object%20Reference) (OtherBodyIndex :type Integer) (bFromSweep :type Boolean) (SweepResult :type Hit%20Result%20Structure%20%28by%20ref%29))
  (bind _rootcomponent (Variables|/Script/Engine.Actor|GetRootComponent OtherActor))
  (bind _returnvalue (Transformation|GetWorldLocation _rootcomponent))
  (Variables|Default|SetExplosed? false)
  (if (not (Variables|Default|GetExplosed?))
    (bind (_outhit _returnvalue_2) (Collision|SphereTraceForObjects _returnvalue (+ _returnvalue (* (Math|Vector|GetForwardVector (Transformation|GetWorldRotation _rootcomponent)) 1e+01)) 2e+02 (Utilities|Array|MakeArray "ObjectTypeQuery3") false 0 "None" true "(R=1.000000,G=0.000000,B=0.000000,A=1.000000)" "(R=0.000000,G=1.000000,B=0.000000,A=1.000000)" 2.0))
    (if _returnvalue_2
      (if (== (.HitActor (Collision|BreakHitResult _outhit)) (Game|Player|GetPlayerPawn 0))
        (Utilities|FlowControl|DoOnce false
          (:Completed
            (Game|Damage|ApplyDamage (.HitActor (Collision|BreakHitResult _outhit)) (Variables|Default|GetBase%20Damage) 0 0)
            (Camera|PlayWorldCameraShake "/Game/Blueprints/Boss_Mecha/CS_Mecha.CS_Mecha_C" (.Location (Collision|BreakHitResult _outhit)) 0.0 1e+04)
            (AddComponent|AddParticleSystemComponent false)
            (Rendering|SetVisibility (Variables|Default|Getr) false false)
            (Audio|PlaySound2D "/Game/VFX/Vefects/Zap_VFX/Audio/SFX_Vefects_Zap_Random_Cue_01.SFX_Vefects_Zap_Random_Cue_01" 1.0 1.0 0.0 0 0)
            (Utilities|FlowControl|Delay 1.5)
            (Actor|DestroyActor)
            (Variables|Default|SetExplosed? true)))))))

(event OnComponentBeginOverlap(w)
  (params (OverlappedComponent :type Primitive%20Component%20Object%20Reference) (OtherActor :type Actor%20Object%20Reference) (OtherComp :type Primitive%20Component%20Object%20Reference) (OtherBodyIndex :type Integer) (bFromSweep :type Boolean) (SweepResult :type Hit%20Result%20Structure%20%28by%20ref%29))
  (if (Actor|ActorHasTag OtherActor "Pillar")
    (Development|PrintString "Hello")
    (CallFunction|EXPLOSION)))

(event Custom|Lock%20On
  (bind _projectilemovement (Variables|Default|GetProjectileMovement))
  (bind _homing_target (CallFunction|FindHomingTarget))
  (Variables|/Script/Engine.ProjectileMovementComponent|SetHomingTargetComponent _projectilemovement _homing_target)
  (Variables|/Script/Engine.ProjectileMovementComponent|SetbIsHomingProjectile _projectilemovement true))

(event Custom|Rotation%20Aim
  (Transformation|SetActorRotation (Math|Rotator|MakeRotator 0.0 0.0 (.yaw (Math|Interpolation|RInterpTo (Transformation|GetActorRotation) (Math|Rotator|FindLookatRotation (Transformation|GetActorLocation) (Transformation|GetActorLocation (Game|Player|GetPlayerPawn 0))) (Utilities|Time|GetWorldDeltaSeconds) 5.0)))))

(event Custom|EXPLOSION
  (bind _returnvalue (Transformation|GetActorLocation))
  (bind _outactors (Actor|GetAllActorswithTag "Mecha"))
  (bind (_outhit _returnvalue_2) (Collision|SphereTraceForObjects _returnvalue _returnvalue 2e+02 (Utilities|Array|MakeArray "ObjectTypeQuery3") false _outactors "None" true "(R=1.000000,G=0.000000,B=0.000000,A=1.000000)" "(R=0.000000,G=1.000000,B=0.000000,A=1.000000)" 2.0))
  (if _returnvalue_2
    (Utilities|FlowControl|DoOnce false
      (:Completed
        (Game|Damage|ApplyDamage (.HitActor (Collision|BreakHitResult _outhit)) (Variables|Default|GetBase%20Damage) 0 0)
        (Camera|PlayWorldCameraShake "/Game/Blueprints/Boss_Mecha/CS_Mecha.CS_Mecha_C" (.Location (Collision|BreakHitResult _outhit)) 0.0 1e+04)
        (AddComponent|AddParticleSystemComponent false)
        (Game|Components|ProjectileMovement|StopSimulating (Variables|Default|GetProjectileMovement) _outhit)
        (Rendering|SetVisibility (Variables|Default|Getr) false false)
        (Audio|PlaySound2D "/Game/VFX/Vefects/Zap_VFX/Audio/SFX_Vefects_Zap_Random_Cue_01.SFX_Vefects_Zap_Random_Cue_01" 1.0 1.0 0.0 0 0)
        (Utilities|FlowControl|Delay 1.5)
        (Actor|DestroyActor)))))

(event EventBeginPlay
  (Audio|PlaySound2D "/Engine/VREditor/Sounds/VR_teleport.VR_teleport" 1.0 1.0 0.0 0 0)
  (bind _returnvalue (Utilities|Time|SetTimerbyEvent (delegate Custom|Rotation%20Aim) 0.01 true))
  (Variables|Default|SetTimerHandle _returnvalue)
  (Utilities|FlowControl|Sequence
    (:then_0
      (CallFunction|Lockon :!label _label)
      (Utilities|FlowControl|Delay 0.5)
      (goto _label))
    (:then_1
      (Utilities|FlowControl|Delay 15.0)
      (CallFunction|EXPLOSION)
      (Actor|DestroyActor))))

(fn ConstructionScript)

(fn FindHomingTarget
  (bind _returnvalue (Game|Player|GetPlayerPawn 0))
  (bind _returnvalue_2 (Game|Player|GetPlayerPawn 0))
  (bind _returnvalue_3 (Transformation|GetActorLocation _returnvalue_2))
  (bind _returnvalue_4 (Transformation|GetActorLocation _returnvalue))
  (bind _returnvalue_5 (- _returnvalue_3 _returnvalue_4))
  (bind _returnvalue_6 (Math|Vector|VectorLength _returnvalue_5))
  (for _array_element (Utilities|Array|MakeArray _returnvalue_2)
    (if (< _returnvalue_6 (Variables|Default|GetClosest%20Distance))
      (Variables|Default|SetClosest%20Distance _returnvalue_6)
      (Variables|/Script/Engine.ProjectileMovementComponent|SetMaxSpeed (Variables|Default|GetProjectileMovement) (Math|Random|RandomFloatinRange 3e+02 6e+02))
      (Variables|Default|SetHoming%20Target%20Test _returnvalue_2)))
  (return (Actor|GetComponentbyClass (Game|Player|GetPlayerPawn 0) "/Script/Engine.SceneComponent")))

(fn MidPointCalculator)

(fn CurveControlPoint)

(fn LocationChara
  (return 0))