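; Mecha boss character with kick, ground-impact and shielded special attacks, a health bar, and a death sequence ending in the victory screen.
; Attack events show zone indicators and play montages whose notifies fire forward sphere traces that damage the player with camera shake.
; Health lives in the Game Instance and feeds the UI on Tick, while the special-attack shield blocks incoming damage.
; BeginPlay sets a blackboard flag after a short delay to start the AI.
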(event Custom|ItsShowTime
  ;[1 0 0.01962] Attacks
  (Utilities|FlowControl|DoOnce false
    (:Completed
      (AI|Components|Blackboard|SetValueasBool (AI|GetBlackboard 0) (Utilities|Name|MakeLiteralName "ItsShowTime?") true)
      (CallFunction|ItsShowTime))))

(event Custom|OnEnnemyDestroy
  (params (DestroyedActor :type Actor%20Object%20Reference))
  ;[0.3979 1 0.399] Begin Play
  (Variables|/Game/Blueprints/Game_Instance.Game_Instance_C|SetHealth_Boss (Variables|Default|GetGiRef) (Math|Float|Clamp(Float) (- (Variables|/Game/Blueprints/Game_Instance.Game_Instance_C|GetHealth_Boss (Variables|Default|GetGiRef)) 2e+01) 0.0 (Variables|/Game/Blueprints/Game_Instance.Game_Instance_C|GetMaxHealthBoss (Variables|Default|GetGiRef)))))

(event Custom|Test
  (Utilities|FlowControl|Delay 4.0)
  (AI|AIMoveTo 0 "-310.000002,190.000000,-12.436511" 0 5.0 false))

(event EventBeginPlay
  ;[0.3979 1 0.399] Begin Play
  (Utilities|FlowControl|Sequence
    (:then_0
      (bind _asgame_instance (Utilities|Casting|CastToGame_Instance (Game|GetGameInstance)))
      (Variables|Default|SetGiRef _asgame_instance)
      (bind _returnvalue (UserInterface|CreateWidget "/Game/Blueprints/UI/WB_BossFightHealth.WB_BossFightHealth_C"))
      (UserInterface|Viewport|AddtoViewport _returnvalue 0)
      (Variables|Default|SetHealth%20UI _returnvalue)
      (for _array_element (Utilities|Array|MakeArray (Actor|ActorHasTag "SPE"))
        (Game|BindEventtoOnDestroyed (delegate Custom|OnEnnemyDestroy))))
    (:then_1
      (Utilities|FlowControl|Delay 0.2)
      (CallFunction|ItsShowTime))))

(event EventAttackZoneImpact
  (bind _attack_impact (Variables|Default|GetAttack%20Impact))
  (bind _returnvalue (Transformation|GetWorldLocation _attack_impact))
  ;[1 0 0.01962] Attacks
  ;;[1 1 1] Attack L
  (if (and (not (Variables|Default|GetisAttacking?)) (not (Variables|Default|GetisDead?)))
    (Animation|Montage|PlayMontage (Variables|Character|GetMesh) "/Game/Dimitry/MECHARIG/Defeated_Montage.Defeated_Montage"
      (:then
        (Rendering|SetVisibility (Variables|Default|GetImpactZone) true false)
        (Variables|Default|SetisAttacking? true)
        (Development|PrintString "Attacking B"))
      (:OnCompleted
        (Rendering|SetVisibility (Variables|Default|GetImpactZone) false false)
        (Variables|Default|SetisAttacking? false))
      (:OnNotifyBegin
        (Rendering|SetVisibility (Variables|Default|GetKickZone) false false)
        (Utilities|FlowControl|Sequence
          (:then_0
            (bind (_outhit _returnvalue_2) (Collision|SphereTraceForObjects _returnvalue (+ _returnvalue (* (Math|Vector|GetForwardVector (Transformation|GetWorldRotation _attack_impact)) 3e+03)) 3.5e+02 (Utilities|Array|MakeArray "ObjectTypeQuery3") false 0 "None"))
            (if _returnvalue_2
              (if (== (.HitActor (Collision|BreakHitResult _outhit)) (Game|Player|GetPlayerPawn 0))
                (Game|Damage|ApplyDamage (.HitActor (Collision|BreakHitResult _outhit)) (Variables|/Game/Blueprints/Game_Instance.Game_Instance_C|GetBossDamage (Variables|Default|GetGiRef)) 0 0)
                (Camera|PlayWorldCameraShake "/Game/Blueprints/Boss_Mecha/CS_Mecha.CS_Mecha_C" (.Location (Collision|BreakHitResult _outhit)) 0.0 1e+04)))))))))

(event EventAttackRightKick
  (bind _attack_position_right_kick (Variables|Default|GetAttack%20Position%20Right%20Kick))
  (bind _returnvalue (Transformation|GetWorldLocation _attack_position_right_kick))
  ;[1 0 0.01962] Attacks
  ;;[1 1 1] Attack R
  (if (and (not (Variables|Default|GetisAttacking?)) (not (Variables|Default|GetisDead?)))
    (Utilities|FlowControl|Delay 2.0)
    (Rendering|SetVisibility (Variables|Default|GetKickZone) true false)
    (Animation|Montage|PlayMontage (Variables|Character|GetMesh) "/Game/Dimitry/MECHARIG/AS_KickFinal.AS_KickFinal"
      (:then
        (Variables|Default|SetisAttacking? true)
        (Development|PrintString "Attacking A"))
      (:OnCompleted
        (Rendering|SetVisibility (Variables|Default|GetKickZone) false false)
        (Variables|Default|SetisAttacking? false))
      (:OnNotifyBegin
        (Rendering|SetVisibility (Variables|Default|GetImpactZone) false false)
        (Utilities|FlowControl|Sequence
          (:then_0
            (bind (_outhit _returnvalue_2) (Collision|SphereTraceForObjects _returnvalue (+ _returnvalue (* (Math|Vector|GetForwardVector (Transformation|GetWorldRotation _attack_position_right_kick)) 3e+03)) 1.4e+02 (Utilities|Array|MakeArray "ObjectTypeQuery3") false 0 "None"))
            (if _returnvalue_2
              (if (== (.HitActor (Collision|BreakHitResult _outhit)) (Game|Player|GetPlayerPawn 0))
                (Game|Damage|ApplyDamage (.HitActor (Collision|BreakHitResult _outhit)) (Variables|/Game/Blueprints/Game_Instance.Game_Instance_C|GetBossDamage (Variables|Default|GetGiRef)) 0 0)
                (Camera|PlayWorldCameraShake "/Game/Blueprints/Boss_Mecha/CS_Mecha.CS_Mecha_C" (.Location (Collision|BreakHitResult _outhit)) 0.0 1e+04)))))))))

(event EventAttackLeftKick
  (bind _attack_position_left_kick (Variables|Default|GetAttack%20Position%20Left%20Kick))
  (bind _returnvalue (Transformation|GetWorldLocation _attack_position_left_kick))
  ;[1 0 0.01962] Attacks
  ;;[1 1 1] Attack L
  (if (and (not (Variables|Default|GetisAttacking?)) (not (Variables|Default|GetisDead?)))
    (Utilities|FlowControl|Delay 2.0)
    (Rendering|SetVisibility (Variables|Default|GetKickZone) true false)
    (Animation|Montage|PlayMontage (Variables|Character|GetMesh) "/Game/Dimitry/MECHARIG/AS_KickFinal.AS_KickFinal"
      (:then
        (Variables|Default|SetisAttacking? true)
        (Development|PrintString "Attacking B"))
      (:OnCompleted
        (Rendering|SetVisibility (Variables|Default|GetKickZone) false false)
        (Variables|Default|SetisAttacking? false))
      (:OnNotifyBegin
        (Utilities|FlowControl|Sequence
          (:then_0
            (bind (_outhit _returnvalue_2) (Collision|SphereTraceForObjects _returnvalue (+ _returnvalue (* (Math|Vector|GetForwardVector (Transformation|GetWorldRotation _attack_position_left_kick)) 3e+03)) 1.4e+02 (Utilities|Array|MakeArray "ObjectTypeQuery3") false 0 "None"))
            (if _returnvalue_2
              (if (== (.HitActor (Collision|BreakHitResult _outhit)) (Game|Player|GetPlayerPawn 0))
                (Game|Damage|ApplyDamage (.HitActor (Collision|BreakHitResult _outhit)) (Variables|/Game/Blueprints/Game_Instance.Game_Instance_C|GetBossDamage (Variables|Default|GetGiRef)) 0 0)
                (Camera|PlayWorldCameraShake "/Game/Blueprints/Boss_Mecha/CS_Mecha.CS_Mecha_C" (.Location (Collision|BreakHitResult _outhit)) 0.0 1e+04)))))))))

(event EventTick
  (params (DeltaSeconds :type Float%20%28single-precision%29))
  (if (not (Variables|Default|GetisDead?))
    (Progress|SetPercent (Variables|/Game/Blueprints/UI/WB_BossFightHealth.WB_BossFightHealth_C|GetHealthBar (Variables|Default|GetHealth%20UI)) (/ (Variables|/Game/Blueprints/Game_Instance.Game_Instance_C|GetHealth_Boss (Variables|Default|GetGiRef)) 3e+03))))

(event Game|Damage|EventAnyDamage
  (params (Damage :type Float%20%28single-precision%29) (DamageType :type Damage%20Type%20Object%20Reference) (InstigatedBy :type Controller%20Object%20Reference) (DamageCauser :type Actor%20Object%20Reference))
  (bind _returnvalue (Game|Player|GetPlayerPawn 0))
  (bind _giref (Variables|Default|GetGiRef))
  (if (not (Variables|Default|GetSpecialAttacking?))
    (Utilities|FlowControl|Sequence
      (:then_0
        ;[0.2458 0.2784 1] Damage
        (Niagara|SpawnSystematLocation "/Game/Blueprints/Boss_Mecha/IA/NS_GotHitMecha.NS_GotHitMecha" (+ (Transformation|GetActorLocation _returnvalue) (* (Transformation|GetActorForwardVector _returnvalue) 1e+02)))
        (Audio|PlaySound2D "/Game/Johann/SFX/SFX_RandomHitBoss.SFX_RandomHitBoss" 1.0 1.0 0.0 0 0)
        (Variables|/Game/Blueprints/Game_Instance.Game_Instance_C|SetHealth_Boss _giref (- (Variables|/Game/Blueprints/Game_Instance.Game_Instance_C|GetHealth_Boss _giref) Damage))
        (if (<= (Variables|/Game/Blueprints/Game_Instance.Game_Instance_C|GetHealth_Boss _giref) 0.0)
          (Pawn|Components|CharacterMovement|DisableMovement (Variables|Character|GetCharacterMovement))
          (Animation|Montage|PlayMontage (Variables|Character|GetMesh) "/Game/Dimitry/MECHARIG/Mutant_Dying_Mecha_Montage.Mutant_Dying_Mecha_Montage"
            (:then
              (Audio|PlaySound2D "/Game/Johann/SFX/mecha-sound-effects-designed-mecha-impact-01-120594.mecha-sound-effects-designed-mecha-impact-01-120594" 1.0 1.0 0.0 0 0)
              (Utilities|FlowControl|Delay 4.0)
              (Rendering|SetVisibility (Variables|Character|GetMesh) false false)
              (Audio|PlaySound2D "/Game/StarterContent/Audio/Explosion02.Explosion02" 1.0 1.0 0.0 0 0)
              (Components|Activation|Activate (Variables|Default|Getdeath) false)
              (Variables|Default|SetisDead? true)
              (Rendering|SetVisibility (Variables|Default|GetKickZone) false false)
              (Utilities|FlowControl|Delay 5.0)
              (Utilities|FlowControl|Sequence
                (:then_0
                  (bind _returnvalue_2 (UserInterface|CreateWidget "/Game/Blueprints/UI/Victory_Screen.Victory_Screen_C"))
                  (UserInterface|Viewport|AddtoViewport _returnvalue_2 0))
                (:then_1
                  (Actor|DestroyActor)))))))
      (:then_1
        (Camera|PlayWorldCameraShake "/Game/Blueprints/Boss_Mecha/CS_HitEnnemy.CS_HitEnnemy_C" (Math|Conversions|ToVector(Float) Damage) 0.0 1e+04)))))

(event EventAttackSpecialStart
  ;[1 0 0.01962] Attacks
  (if true
    (Rendering|SetVisibility (Variables|Default|GetShield) true false)
    (Audio|PlaySound2D "/Engine/EditorSounds/GamePreview/StartSimulate.StartSimulate" 1.0 1.0 0.0 0 0)
    (Variables|Default|SetSpecialAttacking? true)))

(event EventAttackSpecialEnd
  ;[1 0 0.01962] Attacks
  (if true
    (Rendering|SetVisibility (Variables|Default|GetShield) false false)
    (Variables|Default|SetSpecialAttacking? false)))

(fn ConstructionScript)