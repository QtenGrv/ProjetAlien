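; BP_Mecha is the boss mecha actor that moves itself along a spline path in the level.
; On BeginPlay it finds a Path actor and plays a timeline, with play rate set from TimeToCompleteSecs.
; Each update sets location and rotation from the spline, lerping distance from full length to zero so travel runs end to start.
; Tick searches for all Path actors without using the result, and GetPath is an empty stub.
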(event Custom|Move%20Object
  (bind _splinesref (Variables|Default|GetSplinesRef))
  (bind _spline (Variables|/Game/Blueprints/Boss_Mecha/Path.Path_C|GetSpline _splinesref))
  (Components|Timeline|SetPlayRate (Variables|Default|GetMove%20Object%20T) (/ 1.0 (Variables|Default|GetTimeToComplete%28Secs%29)))
  (bind _movetrack (Timeline|Move%20Object%20T Play)
    (:Update
      (Transformation|SetActorTransform (Math|Transform|MakeTransform (Spline|GetLocationatDistanceAlongSpline _spline (Math|Float|Lerp (Spline|GetSplineLength (Variables|/Game/Blueprints/Boss_Mecha/Path.Path_C|GetSpline (Variables|Default|GetSplinesRef))) 0.0 _movetrack) "World") (Spline|GetRotationatDistanceAlongSpline _spline (Math|Float|Lerp (Spline|GetSplineLength (Variables|/Game/Blueprints/Boss_Mecha/Path.Path_C|GetSpline (Variables|Default|GetSplinesRef))) 0.0 _movetrack) "World") "1.000000,1.000000,1.000000")))))

(event EventBeginPlay
  (bind _returnvalue (Actor|GetActorOfClass "/Game/Blueprints/Boss_Mecha/Path.Path_C"))
  (Variables|Default|SetSplinesRef _returnvalue)
  (CallFunction|MoveObject))

(event Collision|EventActorBeginOverlap
  (params (OtherActor :type Actor%20Object%20Reference)))

(event EventTick
  (params (DeltaSeconds :type Float%20%28single-precision%29))
  (Actor|GetAllActorsOfClass "/Game/Blueprints/Boss_Mecha/Path.Path_C"))

(fn ConstructionScript)

(fn GetPath
  (params (Splines :type Array%20of%20Path%20Object%20References)))