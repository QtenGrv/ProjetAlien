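; BP_SpawnBoss is a one-shot trigger that stages the mecha boss's entrance when something overlaps its Rt component.
; The overlap plays a warning sound and briefly spawns two BP_Alarm actors at arrow markers.
; After delays it swaps its spotlight for the BP_LightBoss rect light, animating intensity with a Timeline, then spawns BP_Boss at a billboard and destroys its placeholder mesh and VFX components.
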(event OnComponentBeginOverlap(rt)
  (params (OverlappedComponent :type Primitive%20Component%20Object%20Reference) (OtherActor :type Actor%20Object%20Reference) (OtherComp :type Primitive%20Component%20Object%20Reference) (OtherBodyIndex :type Integer) (bFromSweep :type Boolean) (SweepResult :type Hit%20Result%20Structure%20%28by%20ref%29))
  (Utilities|FlowControl|DoOnce false
    (:Completed
      (Utilities|FlowControl|Sequence
        (:then_0
          (Utilities|FlowControl|DoOnce false
            (:Completed
              (Utilities|FlowControl|Delay 5.0)
              (Game|SpawnActorfromClass "/Game/Blueprints/Boss_Mecha/IA/BP_Boss.BP_Boss_C" (Transformation|GetWorldTransform (Variables|Default|GetBillboard)) "AdjustIfPossibleButAlwaysSpawn" "MultiplyWithRoot" 0 0)
              (Components|DestroyComponent (Variables|Default|GetSkeletalMesh)))))
        (:then_1
          (Utilities|FlowControl|Delay 2.0)
          (bind _returnvalue (Actor|GetActorOfClass "/Game/Johann/BP_LightBoss.BP_LightBoss_C"))
          (Utilities|FlowControl|Sequence
            (:then_0
              (Rendering|SetVisibility (Variables|/Game/Johann/BP_LightBoss.BP_LightBoss_C|GetRectLight _returnvalue) true false)
              (Components|DestroyComponent (Variables|Default|GetSpotLight)))
            (:then_1
              (bind _newtrack_0 (Timeline|Timeline PlayFromStart)
                (:Update
                  (Rendering|Components|Light|SetIntensity (Variables|/Game/Johann/BP_LightBoss.BP_LightBoss_C|GetRectLight _returnvalue) _newtrack_0))))))
        (:then_2
          (Utilities|FlowControl|DoOnce false
            (:Completed
              (Audio|PlaySound2D "/Game/Johann/severe-warning-alarm-98704_Cue.severe-warning-alarm-98704_Cue" 1.0 1.0 0.0 0 0))))
        (:then_3
          (CallFunction|Alarm))))))

(event Custom|Alarm
  (Utilities|FlowControl|Sequence
    (:then_0
      (bind _returnvalue (Game|SpawnActorfromClass "/Game/Johann/BP_Alarm.BP_Alarm_C" (Transformation|GetWorldTransform (Variables|Default|GetArrow1)) "Undefined" "MultiplyWithRoot" 0 0))
      (Utilities|FlowControl|Delay 4.0)
      (Actor|DestroyActor _returnvalue))
    (:then_1
      (bind _returnvalue_2 (Game|SpawnActorfromClass "/Game/Johann/BP_Alarm.BP_Alarm_C" (Transformation|GetWorldTransform (Variables|Default|GetArrow)) "Undefined" "MultiplyWithRoot" 0 0))
      (Utilities|FlowControl|Delay 4.0)
      (Actor|DestroyActor _returnvalue_2))))

(fn ConstructionScript)