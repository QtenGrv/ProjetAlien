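; BP_PillarBoss1 is a destructible pillar actor, filed with the mecha boss assets, with its own health and health bar widget.
; Any damage lowers its health, and the actor destroys itself when health reaches zero.
; Every tick it casts its widget component to WB_PillarHealth and sets the bar from health divided by a hardcoded maximum.
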(event EventBeginPlay)

(event Collision|EventActorBeginOverlap
  (params (OtherActor :type Actor%20Object%20Reference)))

(event EventTick
  (params (DeltaSeconds :type Float%20%28single-precision%29))
  (bind _aswb_pillar_health (Utilities|Casting|CastToWB_PillarHealth (UserInterface|GetWidget (Variables|Default|GetWidget))))
  (Progress|SetPercent (Variables|/Game/Blueprints/Boss_Mecha/IA/WB_PillarHealth.WB_PillarHealth_C|GetHealthBar _aswb_pillar_health) (/ (Variables|Default|GetHealthPillar) 75.0)))

(event Game|Damage|EventAnyDamage
  (params (Damage :type Float%20%28single-precision%29) (DamageType :type Damage%20Type%20Object%20Reference) (InstigatedBy :type Controller%20Object%20Reference) (DamageCauser :type Actor%20Object%20Reference))
  (Variables|Default|SetHealthPillar (- (Variables|Default|GetHealthPillar) Damage))
  (if (<= (Variables|Default|GetHealthPillar) 0.0)
    (Actor|DestroyActor)))

(fn ConstructionScript)