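; Boss gate for the mecha boss that moves vertically once, when an actor first overlaps its trigger box.
; A DoOnce starts a timeline that adds its track value to the mesh's world Z each update, teleporting it, and destroys the scary ambience audio activated at BeginPlay.
; The same trigger plays a 2D door sound and, if the actor is the third-person character, a camera shake on its controller.
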(event OnComponentBeginOverlap(Box)
  (params (OverlappedComponent :type Primitive%20Component%20Object%20Reference) (OtherActor :type Actor%20Object%20Reference) (OtherComp :type Primitive%20Component%20Object%20Reference) (OtherBodyIndex :type Integer) (bFromSweep :type Boolean) (SweepResult :type Hit%20Result%20Structure%20%28by%20ref%29))
  (Utilities|FlowControl|DoOnce false
    (:Completed
      (Utilities|FlowControl|Sequence
        (:then_0
          (bind _newtrack_0 (Timeline|Timeline PlayFromStart)
            (:Update
              _)
            (:Finished
              _))
          (Class|SceneComponent|AddWorldTransform (Variables|Default|GetStaticMesh) (Math|Transform|MakeTransform (Math|Vector|MakeVector 0.0 0.0 _newtrack_0) "0, 0, 0" "1.000000,1.000000,1.000000") false true)
          (Components|DestroyComponent (Variables|Default|Getscarysfxamibance)))
        (:then_1
          (Audio|PlaySound2D "/Game/Johann/SFX/porta-2-tancar-90460.porta-2-tancar-90460" 1.0 1.0 0.0 0 0))
        (:then_2
          (bind _asbp_third_person_character (Utilities|Casting|CastToBP_ThirdPersonCharacter OtherActor))
          (bind _asplayer_controller (Utilities|Casting|CastToPlayerController (Pawn|GetController _asbp_third_person_character)))
          (Game|Feedback|ClientStartCameraShake _asplayer_controller "/Game/Blueprints/Boss_Mecha/CS_DoorMecha.CS_DoorMecha_C" 1.0 "CameraLocal" "0, 0, 0"))))))

(event EventBeginPlay
  (Components|Activation|Activate (Variables|Default|Getscarysfxamibance) false))

(event Collision|EventActorBeginOverlap
  (params (OtherActor :type Actor%20Object%20Reference)))

(event EventTick
  (params (DeltaSeconds :type Float%20%28single-precision%29)))

(fn ConstructionScript)