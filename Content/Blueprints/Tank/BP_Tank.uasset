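; BP_Tank is an actor that plays a short scripted sequence when the third-person character overlaps its capsule.
; The overlap pulls the camera back, plays a pose animation, zeroes gravity and teleports the character to a hardcoded location.
; A parallel delayed branch activates a particle system and starts a Timeline zooming the camera further out.
; Shortly afterwards the tank destroys itself, then sets the character's gravity scale back up.
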(event OnComponentBeginOverlap(Capsule)
  (params (OverlappedComponent :type Primitive%20Component%20Object%20Reference) (OtherActor :type Actor%20Object%20Reference) (OtherComp :type Primitive%20Component%20Object%20Reference) (OtherBodyIndex :type Integer) (bFromSweep :type Boolean) (SweepResult :type Hit%20Result%20Structure%20%28by%20ref%29))
  (bind _asbp_third_person_character (Utilities|Casting|CastToBP_ThirdPersonCharacter OtherActor))
  (Utilities|FlowControl|Sequence
    (:then_0
      (Variables|/Script/Engine.SpringArmComponent|SetTargetArmLength (Variables|/Game/Blueprints/Character/BP_ThirdPersonCharacter.BP_ThirdPersonCharacter_C|GetCameraBoom _asbp_third_person_character) 3e+03)
      (Components|Animation|SetAnimation (Variables|/Script/Engine.Character|GetMesh _asbp_third_person_character) "/Game/Characters/Mannequin_UE4/Animations/Male_Dynamic_Pose1.Male_Dynamic_Pose1")
      (Audio|Components|Audio|Play (Variables|/Script/Engine.Character|GetMesh _asbp_third_person_character) false)
      (Variables|/Script/Engine.CharacterMovementComponent|SetGravityScale (Variables|/Script/Engine.Character|GetCharacterMovement _asbp_third_person_character) 0.0)
      (Transformation|Teleport _asbp_third_person_character "1102.515001,240.076046,125.000000" "0, 0, 0")
      (Utilities|FlowControl|Delay 5.0)
      (Actor|DestroyActor)
      (Variables|/Script/Engine.CharacterMovementComponent|SetGravityScale (Variables|/Script/Engine.Character|GetCharacterMovement _asbp_third_person_character) 1.75))
    (:then_1
      (Utilities|FlowControl|Delay 4.4)
      (Components|Activation|SetActive (Variables|Default|GetParticleSystem) true false)
      (bind _newtrack_0 (Timeline|Timeline PlayFromStart)
        (:Update
          (Variables|/Script/Engine.SpringArmComponent|SetTargetArmLength (Variables|/Game/Blueprints/Character/BP_ThirdPersonCharacter.BP_ThirdPersonCharacter_C|GetCameraBoom _asbp_third_person_character) (Math|Float|Lerp 3e+03 5.5e+03 _newtrack_0)))))))

(event EventBeginPlay)

(event Collision|EventActorBeginOverlap
  (params (OtherActor :type Actor%20Object%20Reference)))

(event EventTick
  (params (DeltaSeconds :type Float%20%28single-precision%29)))

(fn ConstructionScript)