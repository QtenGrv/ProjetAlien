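; Alien_Child is a child Blueprint, apparently of an alien character, with a debug-style M key that fires AddXP with a fixed increment.
; Its BeginPlay and AddXP events are empty, so the key press runs no XP logic in this graph.
; Disconnected leftover nodes hold widget creation and an XP level-up routine that raises LevelSTR, resets XP and prints values, but never execute.
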(event Custom|Add%20XP
  (params (Increment :type Float%20%28double-precision%29)))

(event EventBeginPlay)

(event Collision|EventActorBeginOverlap
  (params (OtherActor :type Actor%20Object%20Reference)))

(event EventTick
  (params (DeltaSeconds :type Float%20%28single-precision%29))
  (|CallParentFunction DeltaSeconds) ; This node is disabled and will not be called.\nDrag off pins to build functionality.
)

(event Input|KeyboardEvents|M
  (params (Key :type Key%20Structure :default "None"))
  (:Pressed
    (CallFunction|AddXP 1e+01)))

(fn ConstructionScript
  (|CallParentFunction))