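; BP_SpawnDEF is a trigger-based spawner that creates a one-time group of Ennemy_DEF actors.
; An overlap with its Box component calls the SPAWN event, which a DoOnce limits to a single run.
; A loop spawns NumberOfEnnemis actors at random horizontal offsets from the spawner's location, adjusting for collisions but always spawning.
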(event OnComponentBeginOverlap(Box)
  (params (OverlappedComponent :type Primitive%20Component%20Object%20Reference) (OtherActor :type Actor%20Object%20Reference) (OtherComp :type Primitive%20Component%20Object%20Reference) (OtherBodyIndex :type Integer) (bFromSweep :type Boolean) (SweepResult :type Hit%20Result%20Structure%20%28by%20ref%29))
  (CallFunction|SPAWN))

(event Custom|SPAWN
  (Utilities|FlowControl|DoOnce false
    (:Completed
      (for _index (range 0 (- (Variables|Default|GetNumberOfEnnemis) 1))
        (Game|SpawnActorfromClass "/Game/Blueprints/Ennemis/Ennemy_DEF.Ennemy_DEF_C" (Math|Conversions|ToTransform(Vector) (+ (Math|Vector|MakeVector (Math|Random|RandomFloatinRange -1e+02 3e+02) (Math|Random|RandomFloatinRange -1e+02 3e+02) 0.0) (Transformation|GetActorLocation))) "AdjustIfPossibleButAlwaysSpawn" "MultiplyWithRoot" 0 0)))))

(fn ConstructionScript)