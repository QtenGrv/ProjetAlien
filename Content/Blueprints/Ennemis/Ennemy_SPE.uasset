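; Ennemy_SPE is an enemy Blueprint that grants SPE XP to the player when killed and weakens the boss.
; AnyDamage clamps Health before subtracting damage; at zero or below it disables movement, calls AddXPSPE on BP_ThirdPersonCharacter and destroys the actor.
; The Destroyed event then lowers HealthBoss on the Projet_Alien game instance by a fixed amount, whatever the cause of destruction.
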(event EventBeginPlay)

(event Collision|EventActorBeginOverlap
  (params (OtherActor :type Actor%20Object%20Reference)))

(event Game|Damage|EventAnyDamage
  (params (Damage :type Float%20%28single-precision%29) (DamageType :type Damage%20Type%20Object%20Reference) (InstigatedBy :type Controller%20Object%20Reference) (DamageCauser :type Actor%20Object%20Reference))
  (Variables|Default|SetHealth (- (Math|Float|Clamp(Float) (Variables|Default|GetHealth) 0.0 (Variables|Default|GetMaxHealth)) Damage))
  (if (<= (Variables|Default|GetHealth) 0.0)
    (Pawn|Components|CharacterMovement|DisableMovement (Variables|Character|GetCharacterMovement))
    (bind _returnvalue (Actor|GetActorOfClass "/Game/Blueprints/Character/BP_ThirdPersonCharacter.BP_ThirdPersonCharacter_C"))
    (Default|AddXPSPE _returnvalue 1e+01)
    (Actor|DestroyActor)))

(event EventTick
  (params (DeltaSeconds :type Float%20%28single-precision%29))
  (|CallParentFunction DeltaSeconds))

(event EventDestroyed
  (bind _asprojet_alien (Utilities|Casting|CastToProjet_Alien (Game|GetGameInstance)))
  (Variables|/Game/Blueprints/Projet_Alien.Projet_Alien_C|SetHealth_Boss _asprojet_alien (- (Variables|/Game/Blueprints/Projet_Alien.Projet_Alien_C|GetHealth_Boss _asprojet_alien) 2e+01)))

(fn ConstructionScript
  (|CallParentFunction))