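; Ennemy_NTR is an enemy actor that displays its health on a bar widget facing the player.
; Each Tick casts HealthBarWidget's widget to Ennemy_UI_NTR and sets its bar from Health over a hardcoded maximum of 60.
; It then rotates the widget component toward the player camera manager's location, billboard-style.
; The construction script only calls its parent, and an EnnemyDEF_UI cast is left unconnected.
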(event EventBeginPlay
  (|CallParentFunction) ; This node is disabled and will not be called.\nDrag off pins to build functionality.
)

(event Collision|EventActorBeginOverlap
  (params (OtherActor :type Actor%20Object%20Reference))
  (|CallParentFunction OtherActor) ; This node is disabled and will not be called.\nDrag off pins to build functionality.
)

(event EventTick
  (params (DeltaSeconds :type Float%20%28single-precision%29))
  (bind _asennemy_ui_ntr (Utilities|Casting|CastToEnnemy_UI_NTR (UserInterface|GetWidget (Variables|Default|GetHealthBar_Widget))))
  (Progress|SetPercent (Variables|/Game/Blueprints/UI/Ennemy_UI_NTR.Ennemy_UI_NTR_C|GetHealthBar _asennemy_ui_ntr) (/ (Variables|Default|GetHealth) 6e+01))
  (Transformation|SetWorldRotation (Variables|Default|GetHealthBar_Widget) (Math|Rotator|FindLookatRotation (Transformation|GetWorldLocation (Variables|Default|GetHealthBar_Widget)) (Transformation|GetWorldLocation (Variables|/Script/Engine.Actor|GetRootComponent (Game|GetPlayerCameraManager 0)))) false false))

(fn ConstructionScript
  (|CallParentFunction))