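; Enemy character with a camera-facing health bar, a montage-driven melee attack and a pool of attack tokens that can be reserved and returned.
; Attack plays a montage whose notify runs a short forward sphere trace, damages the player on a hit and signals attack end.
; On destruction it calls LevelUp and increments the Game Instance's AmountAlive.
; Follow, rotation and overlap-damage events are empty, with older logic left disconnected.
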(event OnComponentBeginOverlap(Mesh)
  (params (OverlappedComponent :type Primitive%20Component%20Object%20Reference) (OtherActor :type Actor%20Object%20Reference) (OtherComp :type Primitive%20Component%20Object%20Reference) (OtherBodyIndex :type Integer) (bFromSweep :type Boolean) (SweepResult :type Hit%20Result%20Structure%20%28by%20ref%29))
  ;[1 1 1] Damage system??
)

(event Custom|FollowPlayer
  ;[1 1 1] FollowPlayer
)

(event Custom|Attack
  ;[1 1 1] Attack System
  (if (not (Animation|Montage|MontageIsPlaying (Components|SkeletalMesh|GetAnimInstance (Variables|Character|GetMesh)) "/Game/Animations/Ennemis/2Hit_EnemyATK_Montage.2Hit_EnemyATK_Montage"))
    (Animation|Montage|PlayMontage (Variables|Character|GetMesh) "/Game/Animations/Ennemis/DEF/AM_BaseAtkSoldat_ATK.AM_BaseAtkSoldat_ATK"
      (:OnNotifyBegin
        (CallFunction|ReachingAttack)
        (Default|CallOnAttackEnd)))
    (else
      (Variables|Default|SetAttackIndex 1))))

(event Custom|ResetAttack
  ;[1 1 1] FollowPlayer
)

(event Custom|DropBonus)

(event Custom|BuffBoss)

(event Custom|ReachingAttack
  (bind _returnvalue (Transformation|GetActorLocation))
  (bind _returnvalue_2 (Transformation|GetActorForwardVector))
  (bind _returnvalue_3 (* _returnvalue_2 1e+02))
  (bind _returnvalue_4 (+ _returnvalue _returnvalue_3))
  ;[1 1 1] Attack System
  (bind _outhit (Collision|SphereTraceForObjects _returnvalue_4 _returnvalue_4 4e+01 (Utilities|Array|MakeArray "ObjectTypeQuery3") false 0 "None"))
  (if (== (.HitActor (Collision|BreakHitResult _outhit)) (Game|Player|GetPlayerPawn 0))
    (Game|Damage|ApplyDamage (.HitActor (Collision|BreakHitResult _outhit)) (Variables|Default|GetBase%20Damage) 0 0)))

(event Custom|Rotation)

(event EventTick
  (params (DeltaSeconds :type Float%20%28single-precision%29))
  (bind _asennemy_ui_ntr (Utilities|Casting|CastToEnnemy_UI_NTR (UserInterface|GetWidget (Variables|Default|GetHealthBar_Widget))))
  (Progress|SetPercent (Variables|/Game/Blueprints/UI/Ennemy_UI_NTR.Ennemy_UI_NTR_C|GetHealthBar _asennemy_ui_ntr) (/ (Variables|Default|GetHealth) 3e+01))
  (Transformation|SetWorldRotation (Variables|Default|GetHealthBar_Widget) (Math|Rotator|FindLookatRotation (Transformation|GetWorldLocation (Variables|Default|GetHealthBar_Widget)) (Transformation|GetWorldLocation (Variables|/Script/Engine.Actor|GetRootComponent (Game|GetPlayerCameraManager 0)))) false false))

(event EventDestroyed
  (CallFunction|LevelUp)
  (bind _asgame_instance (Utilities|Casting|CastToGame_Instance (Game|GetGameInstance)))
  (Variables|/Game/Blueprints/Game_Instance.Game_Instance_C|SetAmount_Alive _asgame_instance (+ (Variables|/Game/Blueprints/Game_Instance.Game_Instance_C|GetAmount_Alive _asgame_instance) 1)))

(event EventReturnToken
  (params (Amount :type Integer))
  (Variables|Default|SetAttackTokensCount (+ (Variables|Default|GetAttackTokensCount) Amount)))

(event EventBeginPlay
  (bind _asgame_instance (Utilities|Casting|CastToGame_Instance (Game|GetGameInstance)))
  (Variables|Default|SetGI_Ref _asgame_instance))

(event EventHiton
  ;[1 1 1] Attack System
)

(fn ConstructionScript)

(fn GetPatrolRoute
  (return 0))

(fn IsAttacking
  (return false))

(fn ReserveToken
  (params (Amount :type Integer))
  (if (>= (Variables|Default|GetAttackTokensCount) Amount)
    (Variables|Default|SetAttackTokensCount (- (Variables|Default|GetAttackTokensCount) Amount))
    (return true)
    (else
      (return false))))

(fn SetMovementSpeed
  (params (Speed :type Float%20%28double-precision%29))
  (bind _output_get (Variables|/Script/Engine.CharacterMovementComponent|SetMaxWalkSpeed (Variables|Character|GetCharacterMovement) Speed))
  (return _output_get))