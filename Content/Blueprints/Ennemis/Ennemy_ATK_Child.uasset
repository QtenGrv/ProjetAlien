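; Child enemy Blueprint, named as an attack variant, that registers with its Salle_Test room and handles its own death.
; On BeginPlay it increments the room's AmountAlive counter through a cast of a stored reference.
; AnyDamage reduces Health, and at zero or below it disables movement and grants XP to the BP_ThirdPersonCharacter found by class lookup.
; It then decrements the room counter and destroys itself, both only if the room cast succeeds.
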(event EventBeginPlay
  (bind _assalle_test (Utilities|Casting|CastToSalle_Test (Variables|Default|GetAs%20Salle%20Test)))
  (Variables|/Game/Cours/Salle_Test.Salle_Test_C|SetAmount%20Alive _assalle_test (+ (Variables|/Game/Cours/Salle_Test.Salle_Test_C|GetAmount%20Alive _assalle_test) 1)))

(event Collision|EventActorBeginOverlap
  (params (OtherActor :type Actor%20Object%20Reference)))

(event Game|Damage|EventAnyDamage
  (params (Damage :type Float%20%28single-precision%29) (DamageType :type Damage%20Type%20Object%20Reference) (InstigatedBy :type Controller%20Object%20Reference) (DamageCauser :type Actor%20Object%20Reference))
  (Variables|Default|SetHealth (- (Math|Float|Clamp(Float) (Variables|Default|GetHealth) 0.0 (Variables|Default|GetMaxHealth)) Damage))
  (if (<= (Variables|Default|GetHealth) 0.0)
    (Pawn|Components|CharacterMovement|DisableMovement (Variables|Character|GetCharacterMovement))
    (bind _returnvalue (Actor|GetActorOfClass "/Game/Blueprints/Character/BP_ThirdPersonCharacter.BP_ThirdPersonCharacter_C"))
    (Default|AddXP _returnvalue 1e+01)
    (bind _assalle_test (Utilities|Casting|CastToSalle_Test (Variables|Default|GetAs%20Salle%20Test)))
    (Variables|/Game/Cours/Salle_Test.Salle_Test_C|SetAmount%20Alive _assalle_test (- (Variables|/Game/Cours/Salle_Test.Salle_Test_C|GetAmount%20Alive _assalle_test) 1))
    (Actor|DestroyActor)))

(event EventTick
  (params (DeltaSeconds :type Float%20%28single-precision%29))
  (|CallParentFunction DeltaSeconds) ; This node is disabled and will not be called.\nDrag off pins to build functionality.
)

(fn ConstructionScript
  (|CallParentFunction))