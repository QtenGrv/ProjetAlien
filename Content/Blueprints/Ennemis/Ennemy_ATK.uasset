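; Melee enemy character that chases the player, attacks, and drops an ATK_Bonus pickup on the ground when killed.
; PawnSensing starts an AI move to the player, then a DoOnce-gated attack montage that resets after playing.
; Hiton, not called in this graph, deals damage via a forward sphere trace.
; Tick updates a camera-facing health bar that assumes 100 max health; BuffBoss and mesh overlap are empty stubs.
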(event OnSeePawn(PawnSensing)
  (params (Pawn :type Pawn%20Object%20Reference))
  ;[1 1 1] FollowPlayer
  (bind _output_get (Variables|Default|SetIsSeeingPlayer?%20 true))
  (if _output_get
    (CallFunction|FollowPlayer)))

(event OnComponentBeginOverlap(Mesh)
  (params (OverlappedComponent :type Primitive%20Component%20Object%20Reference) (OtherActor :type Actor%20Object%20Reference) (OtherComp :type Primitive%20Component%20Object%20Reference) (OtherBodyIndex :type Integer) (bFromSweep :type Boolean) (SweepResult :type Hit%20Result%20Structure%20%28by%20ref%29))
  ;[1 1 1] Damage system??
)

(event Custom|FollowPlayer
  ;[1 1 1] FollowPlayer
  (if (Variables|Default|GetIsSeeingPlayer?%20)
    (AI|AIMoveTo self "0, 0, 0" (Game|GetPlayerCharacter 0) 7e+01 false
      (:OnSuccess
        (Utilities|FlowControl|DoOnce false
          (:Completed
            (CallFunction|Attack)))))))

(event Custom|Attack
  ;[1 1 1] Attack System
  (bind _returnvalue (Animation|PlayAnimMontage self "/Game/Blueprints/Ennemis/Animation/AI/AI_AttackAnim.AI_AttackAnim" 1.0 "None"))
  (Utilities|FlowControl|Delay _returnvalue)
  (CallFunction|ResetAttack))

(event Custom|ResetAttack
  ;[1 1 1] FollowPlayer
  (Utilities|FlowControl|DoOnce false) ; enters at Reset
)

(event Custom|DropBonus
  (bind _returnvalue (Transformation|GetActorLocation))
  (bind _outhit (Collision|LineTraceByChannel _returnvalue (- _returnvalue "0.000000,0.000000,200.000000") "TraceTypeQuery1" false 0 "None"))
  (Game|SpawnActorfromClass "/Game/Blueprints/Bonuses/ATK_Bonus.ATK_Bonus_C" (Math|Transform|MakeTransform (.Location (Collision|BreakHitResult _outhit)) (Math|Rotator|MakeRotator 0.0 0.0 (Math|Random|RandomFloatinRange 0.0 3.6e+02))) "Undefined" "MultiplyWithRoot" 0 0))

(event Custom|BuffBoss)

(event EventTick
  (params (DeltaSeconds :type Float%20%28single-precision%29))
  (bind _healthbar_widget (Variables|Default|GetHealthBar_Widget))
  (bind _asennemy_ui (Utilities|Casting|CastToEnnemy_UI (UserInterface|GetWidget (Variables|Default|GetHealthBar_Widget))))
  (Progress|SetPercent (Variables|/Game/UI/Ennemy_UI.Ennemy_UI_C|GetHealthBar _asennemy_ui) (/ (Variables|Default|GetHealth) 1e+02))
  (Transformation|SetWorldRotation _healthbar_widget (Math|Rotator|FindLookatRotation (Transformation|GetWorldLocation _healthbar_widget) (Transformation|GetWorldLocation (Variables|/Script/Engine.Actor|GetRootComponent (Game|GetPlayerCameraManager 0)))) false false))

(event Game|Damage|EventAnyDamage
  (params (Damage :type Float%20%28single-precision%29) (DamageType :type Damage%20Type%20Object%20Reference) (InstigatedBy :type Controller%20Object%20Reference) (DamageCauser :type Actor%20Object%20Reference))
  (Variables|Default|SetHealth (- (Math|Float|Clamp(Float) (Variables|Default|GetHealth) 0.0 (Variables|Default|GetMaxHealth)) Damage))
  (if (<= (Variables|Default|GetHealth) 0.0)
    (Pawn|Components|CharacterMovement|DisableMovement (Variables|Character|GetCharacterMovement))
    (CallFunction|DropBonus)
    (Actor|DestroyActor)))

(event EventHiton
  (bind _returnvalue (Transformation|GetActorLocation))
  (bind _returnvalue_2 (Transformation|GetActorForwardVector))
  (bind _returnvalue_3 (* _returnvalue_2 1e+02))
  (bind _returnvalue_4 (+ _returnvalue _returnvalue_3))
  ;[1 1 1] Attack System
  (bind _outhit (Collision|SphereTraceForObjects _returnvalue_4 _returnvalue_4 4e+01 (Utilities|Array|MakeArray "ObjectTypeQuery3") false 0 "ForDuration"))
  (if (== (.HitActor (Collision|BreakHitResult _outhit)) (Game|Player|GetPlayerPawn 0))
    (Game|Damage|ApplyDamage (.HitActor (Collision|BreakHitResult _outhit)) 1e+01 0 0)))

(fn ConstructionScript)