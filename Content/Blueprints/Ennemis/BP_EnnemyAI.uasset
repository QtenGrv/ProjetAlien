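; BP_EnnemyAI is an enemy pawn that chases the player on sight and plays a melee attack montage on arrival.
; PawnSensing triggers an AI MoveTo, whose success fires Attack through a DoOnce that resets after the montage's length.
; Mesh overlaps deal random damage to the overlapping actor and print a debug string.
; A separate Hiton event draws a debug sphere trace ahead, but its result is unused.
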(event OnSeePawn(PawnSensing)
  (params (Pawn :type Pawn%20Object%20Reference))
  ;[1 1 1] FollowPlayer
  (bind _output_get (Variables|Default|SetIsSeeingPlayer?%20 true))
  (if _output_get
    (CallFunction|FollowPlayer)))

(event OnComponentBeginOverlap(Mesh)
  (params (OverlappedComponent :type Primitive%20Component%20Object%20Reference) (OtherActor :type Actor%20Object%20Reference) (OtherComp :type Primitive%20Component%20Object%20Reference) (OtherBodyIndex :type Integer) (bFromSweep :type Boolean) (SweepResult :type Hit%20Result%20Structure%20%28by%20ref%29))
  ;[1 1 1] Damage system??
  (Game|Damage|ApplyDamage OtherActor (Math|Random|RandomFloatinRange 1e+01 15.0) 0 self)
  (Development|PrintString "Hello"))

(event Custom|FollowPlayer
  ;[1 1 1] FollowPlayer
  (if (Variables|Default|GetIsSeeingPlayer?%20)
    (AI|AIMoveTo self "0, 0, 0" (Game|GetPlayerCharacter 0) 7e+01 false
      (:OnSuccess
        (Utilities|FlowControl|DoOnce false
          (:Completed
            (CallFunction|Attack)))))))

(event Custom|Attack
  ;[1 1 1] Attack System
  (bind _returnvalue (Animation|PlayAnimMontage self "/Game/Blueprints/Ennemis/Animation/AI/AI_AttackAnim.AI_AttackAnim" 1.0 "None"))
  (Utilities|FlowControl|Delay _returnvalue)
  (CallFunction|ResetAttack))

(event Custom|ResetAttack
  ;[1 1 1] FollowPlayer
  (Utilities|FlowControl|DoOnce false) ; enters at Reset
)

(event EventHiton
  (bind _returnvalue (Transformation|GetActorLocation))
  (bind _returnvalue_2 (Transformation|GetActorForwardVector))
  (bind _returnvalue_3 (* _returnvalue_2 1e+02))
  (bind _returnvalue_4 (+ _returnvalue _returnvalue_3))
  ;[1 1 1] Attack System
  (Collision|SphereTraceForObjects _returnvalue_4 _returnvalue_4 4e+01 (Utilities|Array|MakeArray "ObjectTypeQuery3") false 0 "ForDuration"))

(fn ConstructionScript)