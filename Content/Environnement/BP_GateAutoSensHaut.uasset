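; BP_GateAutoSensHaut is an automatic gate that opens once when its Er trigger component is overlapped.
; Two DoOnce-guarded timelines run from one sequence, each moving a door in X/Y through AddWorldTransform, so track values accumulate as per-update deltas.
; The Door1 timeline also shows GreenLight and activates two particle systems, while the Door timeline hides RedLight.
; No closing or reset logic exists.
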(event OnComponentBeginOverlap(er)
  (params (OverlappedComponent :type Primitive%20Component%20Object%20Reference) (OtherActor :type Actor%20Object%20Reference) (OtherComp :type Primitive%20Component%20Object%20Reference) (OtherBodyIndex :type Integer) (bFromSweep :type Boolean) (SweepResult :type Hit%20Result%20Structure%20%28by%20ref%29))
  (Utilities|FlowControl|Sequence
    (:then_0
      (Utilities|FlowControl|DoOnce false
        (:Completed
          (bind _newtrack_0 (Timeline|Timeline PlayFromStart)
            (:Update
              _)
            (:Finished
              _))
          (Class|SceneComponent|AddWorldTransform (Variables|Default|Getdoor1) (Math|Transform|MakeTransform (Math|Vector|MakeVector (.x _newtrack_0) (.y _newtrack_0) 0.0) "0, 0, 0" "1.000000,1.000000,1.000000") false true)
          (Rendering|SetVisibility (Variables|Default|GetGreen%20Light) true false)
          (Components|Activation|Activate (Variables|Default|GetParticleSystem) false))))
    (:then_1
      (Utilities|FlowControl|DoOnce false
        (:Completed
          (bind _newtrack_0_2 (Timeline|Timeline_0 PlayFromStart)
            (:Update
              _)
            (:Finished
              _))
          (Class|SceneComponent|AddWorldTransform (Variables|Default|Getdoor) (Math|Transform|MakeTransform (Math|Vector|MakeVector (.x _newtrack_0_2) (.y _newtrack_0_2) 0.0) "0, 0, 0" "1.000000,1.000000,1.000000") false true)
          (Rendering|SetVisibility (Variables|Default|GetRed%20Light) false false))))))

(event EventBeginPlay)

(event Collision|EventActorBeginOverlap
  (params (OtherActor :type Actor%20Object%20Reference)))

(event EventTick
  (params (DeltaSeconds :type Float%20%28single-precision%29)))

(fn ConstructionScript)